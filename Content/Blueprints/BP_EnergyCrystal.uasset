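; BP_EnergyCrystal is an energy crystal actor that lights up while the player character is nearby.
; A Sphere component's begin and end overlap events, filtered to BP_ThirdPersonCharacter, drive a Niagara component's parameters.
; Entering turns the crystal color bright blue and raises the particle spawn rate; leaving resets it to dim gray with sparse particles.
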(event OnComponentBeginOverlap(Sphere)
  (params (OverlappedComponent :type Primitive%20Component%20Object%20Reference) (OtherActor :type Actor%20Object%20Reference) (OtherComp :type Primitive%20Component%20Object%20Reference) (OtherBodyIndex :type Integer) (bFromSweep :type Boolean) (SweepResult :type Hit%20Result%20Structure%20%28by%20ref%29))
  (Utilities|Casting|CastToBP_ThirdPersonCharacter OtherActor)
  (Effects|Components|ParticleSystem|SetColorParameter (Variables|Default|GetNiagara) "CrystalColor" "(R=0.001926,G=0.056930,B=1.000000,A=1.000000)")
  (Effects|Components|ParticleSystem|SetFloatParameter (Variables|Default|GetNiagara) "SpawnRate" 5e+01))

(event OnComponentEndOverlap(Sphere)
  (params (OverlappedComponent :type Primitive%20Component%20Object%20Reference) (OtherActor :type Actor%20Object%20Reference) (OtherComp :type Primitive%20Component%20Object%20Reference) (OtherBodyIndex :type Integer))
  (Utilities|Casting|CastToBP_ThirdPersonCharacter OtherActor)
  (Effects|Components|ParticleSystem|SetColorParameter (Variables|Default|GetNiagara) "CrystalColor" "(R=0.098285,G=0.104616,B=0.097165,A=1.000000)")
  (Effects|Components|ParticleSystem|SetFloatParameter (Variables|Default|GetNiagara) "SpawnRate" 5.0))

(fn ConstructionScript)